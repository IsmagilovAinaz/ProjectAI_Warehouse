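; AI forklift robot that hauls pallets to shelves, registering with the task auction manager and refreshing its location, status and battery data every tick.
; Move events use AIMoveTo, then update gameplay tags and blackboard keys that signal the next behavior tree phase.
; Helpers pick the nearest pallet, rotate and slide toward it, attach it to the forklift, and clear tasks.
; Status widget and several helper functions are empty or disconnected.
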(event `StatusHasChanged`
  (`self.ChangeStatusWidget`))

(event `self.ReceiveBeginPlay`
  (bind _robotauction (`self.RobotAuction`))
  (bind _returnvalue (`GameplayStatics.GetActorOfClass` "/Game/__Factory/FactoryNEW_BT.FactoryNEW_BT_C"))
  (set `self.Factory` _returnvalue)
  (bind _returnvalue_2 (`GameplayStatics.GetActorOfClass` "/Game/__Factory/TaskManager/BP_TaskManager.BP_TaskManager_C"))
  (set `self.TaskManager` _returnvalue_2)
  (bind _returnvalue_3 (`GameplayStatics.GetActorOfClass` "/Game/__Factory/TaskManager/BP_TaskAuctionManager.BP_TaskAuctionManager_C"))
  (bind _output_get (set `self.Auction` _returnvalue_3))
  (set `RobotAuctionComponent.RobotID` (`self.RobotID`) _robotauction)
  (`TaskAuctionManager.RegisterRobot` _output_get _robotauction)
  (`self.ChangeStatusWidget`))

(event `self.ReceiveTick`
  (params (DeltaSeconds :type "Float (single-precision)"))
  (bind _robotauction (`self.RobotAuction`))
  (set `RobotAuctionComponent.CurrentLocation` (`self.K2_GetActorLocation`) _robotauction)
  (set `RobotAuctionComponent.CurrentState` (`|GetEnumeratorNameAsString` (`self.RobotStatus`)) _robotauction)
  (set `RobotAuctionComponent.CurrentBatteryLevel` (`self.BatteryLevel`) _robotauction))

(event `MoveToTask`
  (bind (_task_robot _task_pallet) (break `/Game/__Factory/Task/Task_ST` (`self.Task`)))
  (bind _returnvalue (`AIBlueprintHelperLibrary.GetAIController` self))
  (bind _returnvalue_2 (`AIBlueprintHelperLibrary.GetBlackboard` _returnvalue))
  (if (`BlueprintGameplayTagLibrary.HasTag` (`self.TaskTags`) (struct :`TagName` "Status.OnTask"))
    (`self.DrawPathPoints` _returnvalue)
    (`|AIMoveTo` self (`SceneComponent.K2_GetComponentLocation` (`/Game/__Factory/Pawns/Boxes/PalletActor.pointForFork` _task_pallet)) null 10.0
      (:`OnSuccess`
        (set `self.TaskTags` (struct :`GameplayTags` (struct :`(TagName` "ExecTask.TakePallet"))))
        (`BlackboardComponent.SetValueAsBool` _returnvalue_2 "MoveToPallet" false)
        (`BlackboardComponent.SetValueAsBool` _returnvalue_2 "IsAtPallet" true)
        (`BlackboardComponent.SetValueAsBool` _returnvalue_2 "Rotate" true)))))

(event `MoveToShelf`
  (bind (_task_robot _task_pallet _task_shelf) (break `/Game/__Factory/Task/Task_ST` (`self.Task`)))
  (bind _returnvalue (`AIBlueprintHelperLibrary.GetAIController` self))
  (bind _returnvalue_2 (`AIBlueprintHelperLibrary.GetBlackboard` _returnvalue))
  (`|AIMoveTo` self (`SceneComponent.K2_GetComponentLocation` (`/Game/__Factory/Shelf/Shelf_BT.Sphere` _task_shelf)) null 1.0
    (:`then`
      (for _array_element (`AIBlueprintHelperLibrary.GetCurrentPathPoints` _returnvalue)
        _))
    (:`OnSuccess`
      (`BlueprintGameplayTagLibrary.RemoveGameplayTag` (`self.TaskTags`) (struct :`TagName` "ExecTask.MovePallet"))
      (set `self.TaskTags` (struct :`GameplayTags` (struct :`(TagName` "ExecTask.ReleasePallet"))))
      (`BlackboardComponent.SetValueAsBool` _returnvalue_2 "Rotate" true)
      (`BlackboardComponent.SetValueAsBool` _returnvalue_2 "MoveToShelf" false)
      (`BlackboardComponent.SetValueAsBool` _returnvalue_2 "Rotate" true)
      (`BlackboardComponent.SetValueAsVector` _returnvalue_2 "TargetLocation" (`SceneComponent.K2_GetComponentLocation` (`/Game/__Factory/Shelf/Shelf_BT.SlotAnchor_01` _task_shelf))))))

(event `TakePalletEvent`
  (bind (_task_robot _task_pallet) (break `/Game/__Factory/Task/Task_ST` (`self.Task`)))
  (bind _palletpoint (`self.PalletPoint`))
  (bind _staticmesh (`/Game/__Factory/Pawns/Boxes/PalletActor.StaticMesh` _task_pallet))
  (`SceneComponent.K2_SetWorldLocationAndRotation` _staticmesh (`SceneComponent.K2_GetComponentLocation` _palletpoint) (`SceneComponent.K2_GetComponentRotation` _palletpoint) false true)
  (`KismetSystemLibrary.PrintString` (`KismetStringLibrary.Conv_VectorToString` (`SceneComponent.K2_GetComponentLocation` (`/Game/__Factory/Pawns/Boxes/PalletActor.DefaultSceneRoot` _task_pallet))))
  (bind _returnvalue (`SceneComponent.K2_AttachToComponent` _staticmesh (`self.SkeletalMesh`) "Socket1" "SnapToTarget" "SnapToTarget" "KeepWorld" true))
  (if _returnvalue
    (set `self.TaskTags` (struct :`GameplayTags` (struct :`(TagName` "Status.PalletOn"))))))

(event `self.ReceiveActorOnClicked`
  (params (ButtonPressed :type "Key Structure"))
  (`KismetSystemLibrary.PrintString` "Clicked!"))

(fn `ChangeStatusWidget`)

(fn `CheckTask`)

(fn `ClearTask`
  (bind (_emptytask_robot _emptytask_pallet _emptytask_shelf) (break `/Game/__Factory/Task/Task_ST` (`self.EmptyTask`)))
  (set `self.Task` (make `/Game/__Factory/Task/Task_ST` _emptytask_robot _emptytask_pallet _emptytask_shelf))
  (set `self.TaskTags` (struct))
  (set `self.TaskTags` (struct :`GameplayTags` (struct :`(TagName` "Status.Free")))))

(fn `DrawPathPoints`
  (params (AiController :type "AIController Object Reference"))
  (for _array_element (`AIBlueprintHelperLibrary.GetCurrentPathPoints` AiController)
    _))

(fn `FindNearestPallet`
  (params (Pallets :type "Array of /Game/__Factory/Pawns/Boxes/PalletActor Object Reference"))
  (returns (`Nearest pallet` :type "/Game/__Factory/Pawns/Boxes/PalletActor Object Reference"))
  (for _array_element Pallets
    (bind _output_get (set `self.Distance` (`KismetMathLibrary.Vector_Distance` (`SceneComponent.K2_GetComponentLocation` (`self.Mesh`)) (`SceneComponent.K2_GetComponentLocation` (`/Game/__Factory/Pawns/Boxes/PalletActor.pointForFork` _array_element)))))
    (if (< _output_get (`self.MIN_DISTANCE`))
      (set `self.MIN_DISTANCE` _output_get)
      (bind _output_get_2 (set `self.Pallet` _array_element))
      (set `/Game/__Factory/Pawns/Boxes/PalletActor.status` (struct :`GameplayTags` (struct :`(TagName` "Pallet.OnTask"))) _output_get_2)))
  (return _output_get_2))

(fn `GetUnderPallet`
  (bind (_task_robot _task_pallet) (break `/Game/__Factory/Task/Task_ST` (`self.Task`)))
  (`self.K2_AddActorWorldOffset` (* (`self.GetActorForwardVector`) (`KismetMathLibrary.Vector_Distance` (`SceneComponent.K2_GetComponentLocation` (`self.PalletPoint`)) (`SceneComponent.K2_GetComponentLocation` (`/Game/__Factory/Pawns/Boxes/PalletActor.StaticMesh` _task_pallet))))))

(fn `GoToShelf`)

(fn `RotateToPallet`
  (params (Alpha :type "Float (double-precision)"))
  (bind (_task_robot _task_pallet) (break `/Game/__Factory/Task/Task_ST` (`self.Task`)))
  (`self.K2_SetActorRotation` (`KismetMathLibrary.RLerp` (`self.K2_GetActorRotation`) (`KismetMathLibrary.FindLookAtRotation` (`SceneComponent.K2_GetComponentLocation` (`self.SkeletalMesh`)) (`SceneComponent.K2_GetComponentLocation` (`Actor.RootComponent` _task_pallet))) Alpha true)))

(fn `TakePallet`
  (returns (isDone :type Boolean))
  (bind (_task_robot _task_pallet) (break `/Game/__Factory/Task/Task_ST` (`self.Task`)))
  (bind _palletpoint (`self.PalletPoint`))
  (bind _staticmesh (`/Game/__Factory/Pawns/Boxes/PalletActor.StaticMesh` _task_pallet))
  (`self.RotateToPallet` 0.0)
  (`SceneComponent.K2_SetWorldLocationAndRotation` _staticmesh (`SceneComponent.K2_GetComponentLocation` _palletpoint) (`SceneComponent.K2_GetComponentRotation` _palletpoint) false true)
  (`KismetSystemLibrary.PrintString` (`KismetStringLibrary.Conv_VectorToString` (`SceneComponent.K2_GetComponentLocation` (`/Game/__Factory/Pawns/Boxes/PalletActor.DefaultSceneRoot` _task_pallet))))
  (bind _returnvalue (`SceneComponent.K2_AttachToComponent` _staticmesh _palletpoint "Socket1" "SnapToTarget" "SnapToTarget" "SnapToTarget" true))
  (set `self.Pallet` _task_pallet)
  (`KismetSystemLibrary.PrintText` "Hello")
  (return _returnvalue))

(fn `UserConstructionScript`)