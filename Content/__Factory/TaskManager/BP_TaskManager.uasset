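; BP_TaskManager creates, assigns and tracks pallet tasks for AI forklift robots.
; AddTask queues a task and runs RunTaskAllocation, which sends feasible robots' travel-time estimates to TaskAllocationManager and gives the winner the task.
; RunTaskAuction is an uncalled twin using TaskAuctionManager, which also supplies the robot registry.
; RequestTask pops the newest queued task, CompleteTask clears assigned ones, and SortTasks is empty; allocation leaves tasks in the queue.
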(event `self.ReceiveBeginPlay`
  (bind _returnvalue (`GameplayStatics.GetActorOfClass` "/Game/__Factory/TaskManager/BP_TaskAuctionManager.BP_TaskAuctionManager_C"))
  (set `self.TaskAuctionManager` _returnvalue))

(fn `AddTask`
  (params (NewTask :type "/Game/__Factory/Task/S_TaskData Structure (by ref)"))
  (returns (Success :type Boolean) (OutTask :type "/Game/__Factory/Task/S_TaskData Structure"))
  (if (`KismetSystemLibrary.IsValid` NewTask_PalletRef_20_D801DFDB41FE84A5BF526EABF2CD7CEB)
    (bind _returnvalue (`self.GenerateID`))
    (bind _output_get (set `self.Task` (make `/Game/__Factory/Task/S_TaskData` _returnvalue NewTask_Tasktype_18_52F895AB4AFA4109FC758391CEEADE76 NewTask_Priority_19_1424FDBC4179BC8FF76523A0CB1A823E NewTask_PalletRef_20_D801DFDB41FE84A5BF526EABF2CD7CEB NewTask_ShelfRef_21_7CE1B58C448F43F2A519CFAF6E135293 NewTask_TargetNode_22_15B853B549D8EF51A1BE359A8B09C5D9 NewTask_Status_23_E24D9B964060ED44311EBDB517F8A87F (`KismetSystemLibrary.GetGameTimeInSeconds`) NewTask_ShelfSlot_28_EE74D8A946107A69A8FE4EB9509B018B null NewTask_ZonePoint_35_6B81DB034E4BB126E2C685B76B22C1DE)))
    (`KismetArrayLibrary.Array_Add` (`self.TaskQueue`) _output_get)
    (`self.OnTaskAdded` _output_get)
    (`/Engine/EditorBlueprintResources/StandardMacros.IncrementInt` (`self.ActiveTasks`)
      (:`  `
        (`self.RunTaskAllocation` _output_get)
        (return true _output_get)))
    (else
      (return false))))

(fn `CompleteTask`
  (params (Task :type "/Game/__Factory/Task/S_TaskData Structure") (`Task ID` :type String))
  (returns (Success :type Boolean))
  (bind _assignedtasks (`self.AssignedTasks`))
  (bind (_value _returnvalue) (`BlueprintMapLibrary.Map_Find` _assignedtasks `Task ID`))
  (if _returnvalue
    (bind _output_get (set `self.Task` _value))
    (set `self.Task` (make `/Game/__Factory/Task/S_TaskData` (break `/Game/__Factory/Task/S_TaskData` _output_get) (`.Tasktype_18_52F895AB4AFA4109FC758391CEEADE76` (break `/Game/__Factory/Task/S_TaskData` _output_get)) (`.Priority_19_1424FDBC4179BC8FF76523A0CB1A823E` (break `/Game/__Factory/Task/S_TaskData` _output_get)) (`.PalletRef_20_D801DFDB41FE84A5BF526EABF2CD7CEB` (break `/Game/__Factory/Task/S_TaskData` _output_get)) (`.ShelfRef_21_7CE1B58C448F43F2A519CFAF6E135293` (break `/Game/__Factory/Task/S_TaskData` _output_get)) (`.TargetNode_22_15B853B549D8EF51A1BE359A8B09C5D9` (break `/Game/__Factory/Task/S_TaskData` _output_get)) "NewEnumerator2" (`.CreatedTime_24_9D4537FC4DA981198CC3B09B503EFCFD` (break `/Game/__Factory/Task/S_TaskData` _output_get)) 0 null))
    (bind _returnvalue_2 (`BlueprintMapLibrary.Map_Remove` _assignedtasks `Task ID`))
    (if _returnvalue_2
      (`/Engine/EditorBlueprintResources/StandardMacros.DecrementInt` (`self.ActiveTasks`)
        (:`  `
          (`/Engine/EditorBlueprintResources/StandardMacros.IncrementInt` (`self.CompletedTasks`)
            (:`  `
              (return true))))))
    (else
      (return true))))

(fn `GenerateID`
  (returns (ReturnValue :type String))
  (return (`KismetStringLibrary.Concat_StrStr` (`KismetStringLibrary.Concat_StrStr` (`KismetStringLibrary.Concat_StrStr` "TASK_" (`KismetStringLibrary.Conv_IntToString` (`self.ActiveTasks`))) "_") (`KismetStringLibrary.Conv_DoubleToString` (`KismetSystemLibrary.GetGameTimeInSeconds`)))))

(fn `RequestTask`
  (params (RobotRef :type "/Game/Forklifter/AI_Forklifter/BP_AIForklifter Object Reference (by ref)"))
  (returns (OutTask :type "/Game/__Factory/Task/S_TaskData Structure") (Res :type Boolean))
  (bind _taskqueue (`self.TaskQueue`))
  (bind _returnvalue (`KismetArrayLibrary.Array_LastIndex` _taskqueue))
  (bind (_output_taskid _output_tasktype _output_priority _output_palletref _output_shelfref _output_targetnode _output_status _output_createdtime _output_shelfslot _output_robot _output_zonepoint) (break `/Game/__Factory/Task/S_TaskData` (`|GetArrayItem` _taskqueue _returnvalue)))
  (if (> (`KismetArrayLibrary.Array_Length` _taskqueue) 0)
    (bind _output_get (set `self.BestTask` (make `/Game/__Factory/Task/S_TaskData` _output_taskid _output_tasktype _output_priority _output_palletref _output_shelfref _output_targetnode "NewEnumerator1" _output_createdtime _output_shelfslot null _output_zonepoint)))
    (`BlueprintMapLibrary.Map_Add` (`self.AssignedTasks`) _output_taskid _output_get)
    (`KismetArrayLibrary.Array_Remove` _taskqueue _returnvalue)
    (`self.OnTaskAssigned` _output_get)
    (return _output_get true)
    (else
      (return (struct) false))))

(fn `RunTaskAllocation`
  (params (TaskData :type "/Game/__Factory/Task/S_TaskData Structure"))
  (returns (AuctionResult :type "AuctionResult Structure"))
  (bind _returnvalue (`self.K2_GetActorLocation` TaskData_PalletRef_20_D801DFDB41FE84A5BF526EABF2CD7CEB))
  (bind _taskauctionmanager (`self.TaskAuctionManager`))
  (bind _traveltimemap (`self.TravelTimeMap`))
  (for _array_element (`TaskAuctionManager.RegisteredRobots` _taskauctionmanager)
    (if (`RobotAuctionComponent.IsFeasible` _array_element 0.0)
      (`BlueprintMapLibrary.Map_Add` _traveltimemap (`RobotAuctionComponent.RobotID` _array_element) (`RobotAuctionComponent.EstimateTravelTime` _array_element (`self.K2_GetActorLocation` (`ActorComponent.GetOwner` _array_element)) _returnvalue))))
  (bind _returnvalue_2 (`TaskAllocationManager.AllocateTask` (`self.TaskAllocationManager`) TaskData_TaskID_29_D1C7A78646C9CD4B73BB5791A1D967FE _returnvalue (`KismetMathLibrary.Conv_IntToDouble` TaskData_Priority_19_1424FDBC4179BC8FF76523A0CB1A823E) 0.0 _traveltimemap))
  (bind _output_get (set `self.AuctionResultStruct` _returnvalue_2))
  (if (`.bSuccess` (break `AuctionResult` _output_get))
    (bind _returnvalue_3 (`TaskAuctionManager.GetRobotByID` _taskauctionmanager (`.WinnerRobotID` (break `AuctionResult` _output_get))))
    (`RobotAuctionComponent.AddTaskToQueue` _returnvalue_3 (break `AuctionResult` _output_get))
    (bind _asbp_aiforklifter (cast `/Game/Forklifter/AI_Forklifter/BP_AIForklifter` (`ActorComponent.GetOwner` _returnvalue_3)))
    (`BlueprintMapLibrary.Map_Add` (`self.AssignedTasks`) (break `AuctionResult` _output_get) (make `/Game/__Factory/Task/S_TaskData` (break `AuctionResult` _output_get) TaskData_Tasktype_18_52F895AB4AFA4109FC758391CEEADE76 TaskData_Priority_19_1424FDBC4179BC8FF76523A0CB1A823E TaskData_PalletRef_20_D801DFDB41FE84A5BF526EABF2CD7CEB TaskData_ShelfRef_21_7CE1B58C448F43F2A519CFAF6E135293 TaskData_TargetNode_22_15B853B549D8EF51A1BE359A8B09C5D9 TaskData_Status_23_E24D9B964060ED44311EBDB517F8A87F TaskData_CreatedTime_24_9D4537FC4DA981198CC3B09B503EFCFD TaskData_ShelfSlot_28_EE74D8A946107A69A8FE4EB9509B018B _asbp_aiforklifter TaskData_ZonePoint_35_6B81DB034E4BB126E2C685B76B22C1DE))
    (else
      (`KismetSystemLibrary.PrintText` "Allocation failed")))
  (return _returnvalue_2))

(fn `RunTaskAuction`
  (params (TaskData :type "/Game/__Factory/Task/S_TaskData Structure"))
  (returns (AuctionResult :type "AuctionResult Structure"))
  (bind _returnvalue (`self.K2_GetActorLocation` TaskData_PalletRef_20_D801DFDB41FE84A5BF526EABF2CD7CEB))
  (bind _taskauctionmanager (`self.TaskAuctionManager`))
  (bind _traveltimemap (`self.TravelTimeMap`))
  (for _array_element (`TaskAuctionManager.RegisteredRobots` _taskauctionmanager)
    (if (`RobotAuctionComponent.IsFeasible` _array_element 0.0)
      (`BlueprintMapLibrary.Map_Add` _traveltimemap (`RobotAuctionComponent.RobotID` _array_element) (`RobotAuctionComponent.EstimateTravelTime` _array_element (`self.K2_GetActorLocation` (`ActorComponent.GetOwner` _array_element)) _returnvalue))))
  (bind _returnvalue_2 (`TaskAuctionManager.RunAuction` _taskauctionmanager TaskData_TaskID_29_D1C7A78646C9CD4B73BB5791A1D967FE _returnvalue (`KismetMathLibrary.Conv_IntToDouble` TaskData_Priority_19_1424FDBC4179BC8FF76523A0CB1A823E) 0.0 _traveltimemap))
  (bind _output_get (set `self.AuctionResultStruct` _returnvalue_2))
  (if (`.bSuccess` (break `AuctionResult` _output_get))
    (bind _returnvalue_3 (`TaskAuctionManager.GetRobotByID` _taskauctionmanager (`.WinnerRobotID` (break `AuctionResult` _output_get))))
    (`RobotAuctionComponent.AddTaskToQueue` _returnvalue_3 (break `AuctionResult` _output_get))
    (bind _asbp_aiforklifter (cast `/Game/Forklifter/AI_Forklifter/BP_AIForklifter` (`ActorComponent.GetOwner` _returnvalue_3)))
    (`BlueprintMapLibrary.Map_Add` (`self.AssignedTasks`) (break `AuctionResult` _output_get) (make `/Game/__Factory/Task/S_TaskData` (break `AuctionResult` _output_get) TaskData_Tasktype_18_52F895AB4AFA4109FC758391CEEADE76 TaskData_Priority_19_1424FDBC4179BC8FF76523A0CB1A823E TaskData_PalletRef_20_D801DFDB41FE84A5BF526EABF2CD7CEB TaskData_ShelfRef_21_7CE1B58C448F43F2A519CFAF6E135293 TaskData_TargetNode_22_15B853B549D8EF51A1BE359A8B09C5D9 TaskData_Status_23_E24D9B964060ED44311EBDB517F8A87F TaskData_CreatedTime_24_9D4537FC4DA981198CC3B09B503EFCFD TaskData_ShelfSlot_28_EE74D8A946107A69A8FE4EB9509B018B _asbp_aiforklifter TaskData_ZonePoint_35_6B81DB034E4BB126E2C685B76B22C1DE))
    (else
      (`KismetSystemLibrary.PrintText` "Auction failed")))
  (return _returnvalue_2))

(fn `SortTasks`)

(fn `UserConstructionScript`)