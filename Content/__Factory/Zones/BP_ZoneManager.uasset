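; Zone manager actor that tracks loading, unloading and charging zone points in the level and hands out free ones by type.
; On BeginPlay it gathers every BP_ZonePoint and sorts them into three arrays by Type.
; GetFreeZone picks the matching array, and FindFreeZone returns the first point that is free and unreserved, without reserving it.
; GetZoneByType is an unfinished stub.
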(event `self.ReceiveBeginPlay`
  (`self.FillZoneArrays`))

(fn `FillZoneArrays`
  (bind _outactors (`GameplayStatics.GetAllActorsOfClass` "/Game/__Factory/Zones/BP_ZonePoint.BP_ZonePoint_C"))
  (for _array_element _outactors
    (switch `/Game/__Factory/Zones/E_ZoneTypes` (`/Game/__Factory/Zones/BP_ZonePoint.Type` _array_element)
      (:`NewEnumerator0`
        (`KismetArrayLibrary.Array_Add` (`self.LoadingZones`) _array_element))
      (:`NewEnumerator1`
        (`KismetArrayLibrary.Array_Add` (`self.UnloadongZones`) _array_element))
      (:`NewEnumerator2`
        (`KismetArrayLibrary.Array_Add` (`self.CharchingZones`) _array_element)))))

(fn `FindFreeZone`
  (params (Array :type "Array of /Game/__Factory/Zones/BP_ZonePoint Object Reference"))
  (returns (`Array Element` :type "/Game/__Factory/Zones/BP_ZonePoint Object Reference"))
  (for _array_element Array
    (if (and (`/Game/__Factory/Zones/BP_ZonePoint.isFree` _array_element) (not (`/Game/__Factory/Zones/BP_ZonePoint.Reserved` _array_element)))
      (return _array_element))))

(fn `GetFreeZone`
  (params (`Zone Type` :type "/Game/__Factory/Zones/E_ZoneTypes Enum" :default "NewEnumerator0"))
  (returns (`Zone Point` :type "/Game/__Factory/Zones/BP_ZonePoint Object Reference"))
  (switch `/Game/__Factory/Zones/E_ZoneTypes` `Zone Type`
    (:`NewEnumerator0`
      (bind _array_element (`self.FindFreeZone` (`self.LoadingZones`)))
      (return _array_element))
    (:`NewEnumerator1`
      (bind _array_element_2 (`self.FindFreeZone` (`self.UnloadongZones`)))
      (return _array_element_2))
    (:`NewEnumerator2`
      (bind _array_element_3 (`self.FindFreeZone` (`self.CharchingZones`)))
      (return _array_element_3))))

(fn `GetZoneByType`
  (params (ZoneType :type "/Game/__Factory/Zones/E_ZoneTypes Enum" :default "NewEnumerator0"))
  (switch `/Game/__Factory/Zones/E_ZoneTypes` ZoneType))

(fn `UserConstructionScript`)